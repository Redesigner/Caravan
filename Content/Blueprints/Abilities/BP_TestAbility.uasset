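; BP_TestAbility is a test gameplay ability that plays the Melee1 gameplay cue at the hit location and normal when a target is hit.
; On an autonomous proxy, it executes the cue locally through CharacterAbilitySystemComponent, giving the owning client its own feedback.
; For any other role, it executes the cue through the ability with effect context and instigator added.
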(event EventOnTargetHit
  (params (HitResult :type Hit%20Result%20Structure%20%28by%20ref%29))
  (bind (_bblockinghit _binitialoverlap _time _distance _location _impactpoint _normal) (Collision|BreakHitResult HitResult))
  (if (Utilities|Enum|Equal(Enum) (Networking|GetLocalRole (Ability|GetOwningActorfromActorInfo)) "ROLE_AutonomousProxy")
    (bind _ascharacter_ability_system_component (Utilities|Casting|CastToCharacterAbilitySystemComponent (Ability|GetAbilitySystemComponentfromActorInfo)))
    (Class|CharacterAbilitySystemComponent|ExecuteGameplayCueLocal _ascharacter_ability_system_component "(TagName=\"GameplayCue.Melee1\")" (Ability|GameplayCue|MakeGameplayCueParameters :Location _location :Normal _normal))
    (else
      (Class|GameplayAbility|ExecuteGameplayCuewithParams "(TagName=\"GameplayCue.Melee1\")" (Ability|GameplayCue|MakeGameplayCueParameters :EffectContext (Ability|GetContextfromOwner) :Location _location :Normal _normal :Instigator (Components|GetOwner (Ability|GetOwningActorfromActorInfo)))))))