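; TestReticle is a targeting reticle built from two counter-rotating decals that share one dynamic material.
; Fade-in and fade-out events flip a flag that drives a clamped timer on Tick.
; The timer sets the material's opacity and the scale of the second decal.
; Once fully faded out, Tick multicasts a switch to follow-owner movement; a visibility toggle is left disconnected.
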(event EventBeginPlay
  (bind _decal (Variables|Default|GetDecal))
  (Utilities|FlowControl|Sequence
    (:then_0
      (bind _returnvalue (Rendering|Material|CreateDynamicMaterialInstance (Class|DecalComponent|GetDecalMaterial _decal) "None" "None" :!class /Script/Engine.KismetMaterialLibrary))
      (bind _output_get (Variables|Default|SetDecalMaterial _returnvalue))
      (Rendering|Components|Decal|SetDecalMaterial _decal _output_get))
    (:then_1
      (Rendering|Components|Decal|SetDecalMaterial (Variables|Default|GetDecal2) (Variables|Default|GetDecalMaterial)))
    (:then_2
      (Rendering|SetVisibility (Variables|Default|GetDefaultSceneRoot) true true))))

(event EventTick
  (params (DeltaSeconds :type Float%20%28single-precision%29))
  (Utilities|FlowControl|Sequence
    (:then_0
      (Transformation|AddWorldRotation (Variables|Default|GetDecal2) (* "0,90.000000,0" DeltaSeconds) false true)
      (Transformation|AddWorldRotation (Variables|Default|GetDecal) (* "0,-45.000000,0" DeltaSeconds) false true))
    (:then_1
      (bind _output_get (Variables|Default|SetCurrentFadeTime (Math|Float|Clamp(Float) (+ (Variables|Default|GetCurrentFadeTime) (select (Variables|Default|GetFadingIn) (* DeltaSeconds -1.0) DeltaSeconds)) 0.0 (Variables|Default|GetFadeTime))))
      (Rendering|Material|SetScalarParameterValue (Variables|Default|GetDecalMaterial) "Opacity" (- 1.0 (Math|Float|Clamp(Float) (/ _output_get (Variables|Default|GetFadeTime)))) :!class /Script/Engine.MaterialInstanceDynamic)
      (Transformation|SetRelativeScale3D (Variables|Default|GetDecal2) (Math|Conversions|ToVector(Float) (- 1.0 (Math|Float|Clamp(Float) (/ _output_get (Variables|Default|GetFadeTime)))))))
    (:then_2
      (if (not (not (>= (Variables|Default|GetCurrentFadeTime) (Variables|Default|GetFadeTime))))
        (Class|TargetingReticleActor|MulticastSetReticleMovementMode "FollowOnwer")))))

(event EventOnFadeOut
  (Variables|Default|SetFadingIn false))

(event EventOnFadein
  (Variables|Default|SetFadingIn true))

(fn ConstructionScript)