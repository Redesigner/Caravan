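; Character Blueprint that handles Gameplay Ability System cues for spell casting, melee hits and fire effects.
; CastSpell toggles a CastingSpell flag, while FireEffect1 spawns a fireball Niagara system at the effect context's origin.
; Melee1 spawns a directional hit-shock effect and briefly nudges the camera boom, resetting it by timer.
; Melee1 filters on instigator validity and net role, separating autonomous-proxy cues from authoritative ones.
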(event EventBeginPlay)

(event Collision|EventActorBeginOverlap
  (params (OtherActor :type Actor%20Object%20Reference)))

(event EventGameplayCue.CastSpell
  (params (EventType :type EGameplayCueEvent%20Enum :default "OnActive") (Parameters :type Gameplay%20Cue%20Parameters%20Structure%20%28by%20ref%29))
  (switch Utilities|FlowControl|Switch|SwitchonEGameplayCueEvent EventType
    (:OnActive
      (Variables|Default|SetCastingSpell true))
    (:Removed
      (Variables|Default|SetCastingSpell false))))

(event EventGameplayCue.Melee1
  (params (EventType :type EGameplayCueEvent%20Enum :default "OnActive") (Parameters :type Gameplay%20Cue%20Parameters%20Structure%20%28by%20ref%29))
  (bind (_normalizedmagnitude _rawmagnitude _effectcontext _matchedtagname _originaltag _aggregatedsourcetags _aggregatedtargettags _location _normal _instigator) (Ability|GameplayCue|BreakGameplayCueParameters Parameters))
  (bind _returnvalue (Networking|GetLocalRole))
  (bind _returnvalue_2 (Utilities|Enum|Equal(Enum) _returnvalue "ROLE_AutonomousProxy"))
  (if (Utilities|Enum|Equal(Enum) EventType "Executed")
    (Utilities|IsValid _instigator
      (:Is%20Valid
        (if _returnvalue_2
          (bind _returnvalue_3 (Niagara|SpawnSystematLocation "/Game/ParticleEffects/NS_HitShock.NS_HitShock" _location :!label _label))
          (Niagara|SetNiagaraVariable(Vector3) _returnvalue_3 "Direction" _normal)
          (Variables|/Script/Engine.SpringArmComponent|SetTargetOffset (Variables|Default|GetCameraBoom) (* _normal 5.0))
          (Utilities|Time|SetTimerbyFunctionName 0 "ResetCameraOffset" 0.05)))
      (:Is%20Not%20Valid
        (if (not _returnvalue_2)
          (goto _label))))))

(event EventGameplayCue.FireEffect1
  (params (EventType :type EGameplayCueEvent%20Enum :default "OnActive") (Parameters :type Gameplay%20Cue%20Parameters%20Structure%20%28by%20ref%29))
  (switch Utilities|FlowControl|Switch|SwitchonEGameplayCueEvent EventType
    (:Executed
      (Niagara|SpawnSystematLocation "/Game/ParticleEffects/NS_Fireball.NS_Fireball" (Class|AbilitySystemBlueprintLibrary|EffectContextGetOrigin (.EffectContext (Ability|GameplayCue|BreakGameplayCueParameters Parameters)))))))

(fn ConstructionScript)

(fn ResetCameraOffset
  (Variables|/Script/Engine.SpringArmComponent|SetTargetOffset (Variables|Default|GetCameraBoom) "0, 0, 0"))