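; CharacterBase_BP is a base character Blueprint that shows a red health bar on a material billboard.
; The construction script creates a dynamic instance of M_ProgressBar, starting full.
; Every Tick polls a gameplay attribute from the AbilitySystem and writes it to the bar's Percentage parameter, assuming a fixed maximum of 100.
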(event EventBeginPlay)

(event Collision|EventActorBeginOverlap
  (params (OtherActor :type Actor%20Object%20Reference)))

(event EventTick
  (params (DeltaSeconds :type Float%20%28single-precision%29))
  (Rendering|Material|SetScalarParameterValue (Variables|Default|GetHealth%20Bar%20Material%20Instance) "Percentage" (/ (.ReturnValue (Class|AbilitySystemComponent|GetGameplayAttributeValue (Variables|Default|GetAbilitySystem) "(AttributeName=\"CurrentHealth\",Attribute=/Script/CaravanAbility.CharacterBaseAttributeSet:CurrentHealth,AttributeOwner=Class'\"/Script/CaravanAbility.CharacterBaseAttributeSet\"')")) 1e+02) :!class /Script/Engine.MaterialInstanceDynamic))

(fn ConstructionScript
  (bind _returnvalue (Rendering|Material|CreateDynamicMaterialInstance (Variables|Default|GetMaterialBillboard) 0 "/Game/Materials/M_ProgressBar.M_ProgressBar" "None" :!class /Script/Engine.PrimitiveComponent))
  (bind _output_get (Variables|Default|SetHealth%20Bar%20Material%20Instance _returnvalue))
  (Rendering|Material|SetScalarParameterValue _output_get "Percentage" 1.0 :!class /Script/Engine.MaterialInstanceDynamic)
  (Rendering|Material|SetVectorParameterValue _output_get "Base Color" "(R=1.000000,G=0.000000,B=0.000000,A=1.000000)" :!class /Script/Engine.MaterialInstanceDynamic))