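; PlayerControllerBase is a player controller Blueprint with unfinished or disabled logic for showing and hiding a dialog widget.
; BeginPlay is empty, and both dialog chains are disconnected, so neither runs.
; One chain would hide the widget and clear DisplayingDialog.
; The other would create a widget for the local player, but it names no class and sets DialogWidget to None before hiding it and adding it to the viewport.
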(event EventBeginPlay)

(event Input|ActionEvents|InputActionInteract
  (params (Key :type Key%20Structure)))

(fn ConstructionScript)